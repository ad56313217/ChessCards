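; Client actor that tests a TCP-style socket connection to a local server from keyboard input.
; On BeginPlay it enables player input; C opens a socket to localhost and starts a looping one-second timer that polls for received messages and prints them.
; V sends a fixed greeting string and prints a confirmation.
; Socket work relies on custom SocketCreate, SocketSend and SocketReceive functions.
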(event Custom|Receive
  (bind (_breceive _recvmessage) (Class|TCPSocketClient|SocketReceive))
  (Development|PrintString (Utilities|String|Append "Receive?:" (Utilities|String|ToString(Boolean) _breceive) "| receiveStr: " _recvmessage)))

(event EventBeginPlay
  (Input|EnableInput (Game|GetPlayerController 0)))

(event Collision|EventActorBeginOverlap
  (params (OtherActor :type Actor%20Object%20Reference)))

(event EventTick
  (params (DeltaSeconds :type Float%20%28single-precision%29)))

(event Input|KeyboardEvents|C
  (params (Key :type Key%20Structure))
  (:Pressed
    (Class|TCPSocketClient|SocketCreate "127.0.0.1" 8888)
    (Utilities|Time|SetTimerbyEvent (delegate Custom|Receive) 1.0 true)))

(event Input|KeyboardEvents|V
  (params (Key :type Key%20Structure))
  (:Pressed
    (Class|TCPSocketClient|SocketSend "I am Client 棋牌123")
    (Development|PrintString "Send I am Client  棋牌")))

(fn ConstructionScript)