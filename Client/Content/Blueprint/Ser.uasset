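; Test actor that acts as a TCP server, driven by keyboard input enabled for player 0 on BeginPlay.
; S chains create, bind, listen and accept socket calls with hardcoded addresses, printing the name of any failed step.
; A successful accept sets a zero-time, non-looping timer on RECVData, whose only action is a receive call.
; D sends a fixed greeting string and prints a debug message.
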(event Custom|RECVData
  (Class|TCPSocketServer|RecvSoc))

(event EventBeginPlay
  (Input|EnableInput (Game|GetPlayerController 0)))

(event Collision|EventActorBeginOverlap
  (params (OtherActor :type Actor%20Object%20Reference)))

(event EventTick
  (params (DeltaSeconds :type Float%20%28single-precision%29)))

(event Input|KeyboardEvents|S
  (params (Key :type Key%20Structure))
  (:Pressed
    (bind _returnvalue (Class|TCPSocketServer|CreateSoc))
    (if _returnvalue
      (bind _returnvalue_2 (Class|TCPSocketServer|BindSoc "0.0.0.0" 4303))
      (if _returnvalue_2
        (bind _returnvalue_3 (Class|TCPSocketServer|ListenSoc 1))
        (if _returnvalue_3
          (bind _returnvalue_4 (Class|TCPSocketServer|AcceptSoc "127.0.0.1" 8888))
          (if _returnvalue_4
            (Utilities|Time|SetTimerbyEvent (delegate Custom|RECVData) 0.0)
            (else
              (Development|PrintString "Accept Soc")))
          (else
            (Development|PrintString "Listen Soc")))
        (else
          (Development|PrintString "Bind Soc")))
      (else
        (Development|PrintString "Create Soc")))))

(event Input|KeyboardEvents|D
  (params (Key :type Key%20Structure))
  (:Pressed
    (Class|TCPSocketServer|SendSoc "i am tcp server")
    (Development|PrintString "Send Mes")))

(fn ConstructionScript)